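; SG_coding2 is a save-game Blueprint, judging by its name, that restores collected coin and door state.
; LoadCollectedCoins calls LoadCollectedState on each valid object in CollectedCoins, or prints a message when the array is empty.
; LoadDoorStates calls LoadDoorState on the single CamDoorTrigger reference without a validity check.
; Both functions delegate the restoration to the referenced objects.
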(fn `LoadCollectedCoins`
  (if (> (`KismetArrayLibrary.Array_Length` (`self.CollectedCoins`)) 0)
    (for _array_element (`self.CollectedCoins`)
      (`/Engine/EditorBlueprintResources/StandardMacros.IsValid` _array_element
        (:`Is Valid`
          (`/Game/Blueprints/BP_Coin.Load Collected State` _array_element))))
    (else
      (`KismetSystemLibrary.PrintString` null "No collected coins to load" false))))

(fn `LoadDoorStates`
  (`/Game/Blueprints/BP_CamDoorTrigger.LoadDoorState` (`self.CamDoorTrigger`)))
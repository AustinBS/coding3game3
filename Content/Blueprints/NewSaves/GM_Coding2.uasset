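; GM_Coding2 is a game mode that manages per-level saves using SG_coding2 objects, with the level name as the slot.
; BeginPlay loads or creates the save, restores collected coins, door states and any non-zero player transform, and deletes saves that fail the cast.
; Checkpoint stores the player transform and saves; LevelFinished clears the transform and CamDoorTrigger, then saves.
; Older stamina and ability save/load logic remains but never runs.
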(event `SaveGame`
  ;[1 1 1] Old Saving and Loading methods
)

(event `LoadGame`
  ;[1 1 1] Old Saving and Loading methods
)

(event `DeleteGame`
  ;[1 1 1] Old Saving and Loading methods
)

(event `self.ReceiveBeginPlay`
  (bind _playertransform_location (`KismetMathLibrary.BreakTransform` (`/Game/Blueprints/NewSaves/SG_coding2.PlayerTransform` (`self.LevelSave`))))
  (`KismetSystemLibrary.PrintString` "Loaded into GM_Coding2 Game Mode")
  (bind _returnvalue (`GameplayStatics.GetCurrentLevelName` true))
  (bind _returnvalue_2 (`GameplayStatics.DoesSaveGameExist` _returnvalue))
  (if _returnvalue_2
    (bind _returnvalue_3 (`GameplayStatics.LoadGameFromSlot` _returnvalue))
    (bind _assg_coding_2 (cast `/Game/Blueprints/NewSaves/SG_coding2` _returnvalue_3)
      (:`then`
        (bind _output_get (set `self.LevelSave` _assg_coding_2))
        (`/Game/Blueprints/NewSaves/SG_coding2.LoadCollectedCoins` _output_get)
        (`/Game/Blueprints/NewSaves/SG_coding2.LoadDoorStates` _output_get)
        ;[1 1 1] if location not === 0,0,0
        ; then set it to that
        (if (not (`KismetMathLibrary.EqualExactly_VectorVector` _playertransform_location))
          (`SceneComponent.K2_SetWorldTransform` (`Character.CapsuleComponent` (`GameplayStatics.GetPlayerCharacter` 0)) (`/Game/Blueprints/NewSaves/SG_coding2.PlayerTransform` (`self.LevelSave`)) false false)))
      (:`CastFailed`
        ;[1 1 1] Deleting Save Game
        (`KismetSystemLibrary.PrintString` "Cast to SG_coding2 failed, deleting")
        (`GameplayStatics.DeleteGameInSlot` _returnvalue)))
    (else
      ;[1 1 1] New Save Game
      (bind _returnvalue_4 (`GameplayStatics.CreateSaveGameObject` "/Game/Blueprints/NewSaves/SG_coding2.SG_coding2_C"))
      (set `self.LevelSave` _returnvalue_4)
      (`KismetSystemLibrary.PrintString` "Created new SG_coding2"))))

(event `Save Game`
  (bind _returnvalue (`GameplayStatics.GetCurrentLevelName` true))
  (bind _returnvalue_2 (`GameplayStatics.SaveGameToSlot` (`self.LevelSave`) _returnvalue))
  (if _returnvalue_2
    (`KismetSystemLibrary.PrintString` "saved level")
    (else
      (`KismetSystemLibrary.PrintString` "No level saved"))))

(fn `Checkpoint`
  (params (`Player Transform` :type "Transform Structure"))
  (set `/Game/Blueprints/NewSaves/SG_coding2.PlayerTransform` `Player Transform` (`self.LevelSave`))
  (`self.Save Game`))

(fn `LevelFinished`
  (bind _levelsave (`self.LevelSave`))
  (set `/Game/Blueprints/NewSaves/SG_coding2.PlayerTransform` (struct) _levelsave)
  (set `/Game/Blueprints/NewSaves/SG_coding2.CamDoorTrigger` null _levelsave)
  (`KismetSystemLibrary.PrintString` "Level Finished" true true (struct :`R` 1.0 :`B` 0.850331 :`A` 1.0) 5.0)
  (`self.Save Game`))

(fn `UserConstructionScript`)
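; Game instance that handles saving and loading of third-person player state through an SG_coding2 save object in a named slot.
; SaveGame reuses or creates the save object, copies the character's stamina, capsule transform, sprint and shoot flags into it, then writes the slot.
; LoadGame reads an existing slot, but assigns each saved field back to itself, so nothing is applied to the character despite the success message.
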(event `SaveGame`
  (`KismetSystemLibrary.PrintString` "Starting Save Game")
  (bind _returnvalue (`GameplayStatics.DoesSaveGameExist` (`self.Slot Name`)))
  (if _returnvalue
    (bind _returnvalue_2 (`GameplayStatics.LoadGameFromSlot` (`self.Slot Name`)))
    (set `self.Saver Subclass` _returnvalue_2)
    (else
      (bind _returnvalue_3 (`GameplayStatics.CreateSaveGameObject` "/Game/Blueprints/SG_coding2.SG_coding2_C"))
      (set `self.Saver Subclass` _returnvalue_3)))
  (bind _assg_coding_2 (cast `/Game/Blueprints/SG_coding2` (`self.Saver Subclass`)))
  (bind _asbp_third_person_character (cast `/Game/ThirdPerson/Blueprints/BP_ThirdPersonCharacter` (`GameplayStatics.GetPlayerCharacter` 0)))
  (set `/Game/Blueprints/SG_coding2.PlayerStamina` (`/Game/ThirdPerson/Blueprints/BP_ThirdPersonCharacter.Stamina` _asbp_third_person_character) _assg_coding_2)
  (set `/Game/Blueprints/SG_coding2.PlayerTransform` (`SceneComponent.K2_GetComponentToWorld` (`Character.CapsuleComponent` _asbp_third_person_character)) _assg_coding_2)
  (set `/Game/Blueprints/SG_coding2.PlayerCanSprint` (`/Game/ThirdPerson/Blueprints/BP_ThirdPersonCharacter.CanSprint` _asbp_third_person_character) _assg_coding_2)
  (set `/Game/Blueprints/SG_coding2.PlayerCanShoot` (`/Game/ThirdPerson/Blueprints/BP_ThirdPersonCharacter.CanShoot` _asbp_third_person_character) _assg_coding_2)
  (`GameplayStatics.SaveGameToSlot` _assg_coding_2 (`self.Slot Name`))
  (`KismetSystemLibrary.PrintString` "game saved successfully"))

(event `LoadGame`
  (`KismetSystemLibrary.PrintString` "Starting Load Game")
  (bind _returnvalue (`GameplayStatics.DoesSaveGameExist` (`self.Slot Name`)))
  (if _returnvalue
    (bind _returnvalue_2 (`GameplayStatics.LoadGameFromSlot` (`self.Slot Name`)))
    (bind _assg_coding_2 (cast `/Game/Blueprints/SG_coding2` _returnvalue_2))
    (cast `/Game/ThirdPerson/Blueprints/BP_ThirdPersonCharacter` (`GameplayStatics.GetPlayerCharacter` 0))
    (set `/Game/Blueprints/SG_coding2.PlayerStamina` (`/Game/Blueprints/SG_coding2.PlayerStamina` _assg_coding_2) _assg_coding_2)
    (bind _output_get (set `/Game/Blueprints/SG_coding2.PlayerTransform` (`/Game/Blueprints/SG_coding2.PlayerTransform` _assg_coding_2) _assg_coding_2))
    (set `/Game/Blueprints/SG_coding2.PlayerCanSprint` (`/Game/Blueprints/SG_coding2.PlayerCanSprint` _assg_coding_2) _assg_coding_2)
    (set `/Game/Blueprints/SG_coding2.PlayerCanShoot` (`/Game/Blueprints/SG_coding2.PlayerCanShoot` _assg_coding_2) _assg_coding_2)
    (set `/Game/Blueprints/SG_coding2.PlayerTransform` _output_get _assg_coding_2)
    (`KismetSystemLibrary.PrintString` "Loading Successful")))
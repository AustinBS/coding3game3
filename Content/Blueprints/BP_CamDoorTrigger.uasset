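; BP_CamDoorTrigger is a one-shot trigger that opens the level's BP_CameraDoor when the third-person character enters its sphere.
; On overlap it passes the player to OpenDoor, destroys its sphere and records itself in the GM_Coding2 game mode's LevelSave.
; LoadDoorState restores the triggered state by removing the sphere and calling LoadDoorState on the door, which is found by class lookup.
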(event `self.Sphere1.OnComponentBeginOverlap`
  (params (OverlappedComponent :type "PrimitiveComponent Object Reference") (OtherActor :type "Actor Object Reference") (OtherComp :type "PrimitiveComponent Object Reference") (OtherBodyIndex :type Integer) (bFromSweep :type Boolean) (SweepResult :type "HitResult Structure (by ref)"))
  (cast `/Game/ThirdPerson/Blueprints/BP_ThirdPersonCharacter` OtherActor)
  (bind _returnvalue (`GameplayStatics.GetActorOfClass` "/Game/Blueprints/BP_CameraDoor.BP_CameraDoor_C"))
  (`/Game/Blueprints/BP_CameraDoor.OpenDoor` _returnvalue OtherActor) ; new view target is the player
  (`ActorComponent.K2_DestroyComponent` (`self.Sphere1`))
  (bind _asgm_coding_2 (cast `/Game/Blueprints/NewSaves/GM_Coding2` (`GameplayStatics.GetGameMode`)))
  (set `/Game/Blueprints/NewSaves/SG_coding2.CamDoorTrigger` self (`/Game/Blueprints/NewSaves/GM_Coding2.LevelSave` _asgm_coding_2)))

(event `LoadDoorState`
  (`ActorComponent.K2_DestroyComponent` (`self.Sphere1`))
  (bind _returnvalue (`GameplayStatics.GetActorOfClass` "/Game/Blueprints/BP_CameraDoor.BP_CameraDoor_C"))
  (`/Game/Blueprints/BP_CameraDoor.LoadDoorState` _returnvalue))

(fn `UserConstructionScript`)
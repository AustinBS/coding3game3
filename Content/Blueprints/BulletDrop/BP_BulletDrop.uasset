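; Test actor that simulates and draws a bullet drop trajectory from its Arrow component, alongside Unreal's built-in projectile path prediction.
; BulletDropCalculator steps through line-trace segments, adding gravity scaled by simulation frequency, until a hit or the step count runs out, then resets start and velocity.
; From BeginPlay, both the manual calculation and PredictProjectilePath repeat every 0.2 seconds with debug drawing.
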(event `Bullet Drop Calculator`
  (set `self.End` (+ (`self.Start`) (/ (`self.Velocity`) (`KismetMathLibrary.MakeVector` (`self.Sim Frequency`) 1.0 1.0))))
  (for _ (range 1 (+ (`KismetMathLibrary.FTrunc` (`self.Sim Frequency`)) 1))
    (`KismetSystemLibrary.DrawDebugLine` (`self.Start`) (`self.End`) (struct :`R` 0.996226 :`B` 1.0 :`A` 1.0) (`self.Max Sim time`))
    (`KismetSystemLibrary.DrawDebugSphere` (`self.End`) 5.0 12 (struct :`R` 0.274832 :`G` 0.92425 :`B` 1.0 :`A` 1.0) (`self.Max Sim time`))
    (bind (_outhit _returnvalue) (`KismetSystemLibrary.LineTraceSingleByProfile` :`Start` (`self.Start`) :`End` (`self.End`) :`ProfileName` "BlockAll" :`DrawDebugType` "ForDuration"))
    (if _returnvalue
      (`KismetSystemLibrary.PrintString` "we hit something")
      (break)
      (else
        (set `self.Start` (`self.End`))
        ;[1 1 1] add gravity to velocity
        (set `self.Velocity` (+ (`self.Velocity`) (`KismetMathLibrary.MakeVector` 0.0 0.0 (/ -980.0 (`KismetMathLibrary.Square` (`self.Sim Frequency`))))))
        ;[1 1 1] set end to the new start position plus velocity
        (set `self.End` (+ (`self.Start`) (/ (`self.Velocity`) (`KismetMathLibrary.MakeVector` (`self.Sim Frequency`) 1.0 1.0)))))))
  ;[1 1 1] reset start and velocity when complete
  (set `self.Start` (`SceneComponent.K2_GetComponentLocation` (`self.Arrow`)))
  (set `self.Velocity` (1200.0 0.0 0.0)))

(event `self.ReceiveBeginPlay`
  (bind _output_get (set `self.Start` (`SceneComponent.K2_GetComponentLocation` (`self.Arrow`))))
  (`|ExecutionSequence` :!label _label
    (:`then_0`
      (`self.Bullet Drop Calculator`))
    (:`then_1`
      (`GameplayStatics.Blueprint_PredictProjectilePath_Advanced` (make `PredictProjectilePathParams` _output_get (`self.startingVelocity`) true 0.0 (`self.Max Sim time`) true "ECC_WorldStatic" _ _ (`self.Sim Frequency`) 0.0 "ForDuration"))
      (`KismetSystemLibrary.Delay` 0.2)
      (goto _label))))

(fn `UserConstructionScript`)